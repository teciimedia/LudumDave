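; BP_Dam is the dam actor, which holds a health value and has a health widget.
; On BeginPlay it passes itself to the DamHP widget and binds Phase2Damage to a dispatcher on the player's BP_Hero.
; Phase2Damage currently only prints a message, without changing health.
; TakeDamage and Heal clamp health between fixed bounds and store a normalized HealthPercent, but neither is called in this Blueprint.
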(event `self.ReceiveBeginPlay`
  (bind _asdam_hp (cast `/Game/UI/DamHP` (`WidgetComponent.GetUserWidgetObject` (`self.HealthUI`))))
  ;[1 1 1] Dispatcher from Hero BP to call for Phase 2 Damage to start
  (set `/Game/UI/DamHP.Dam` self _asdam_hp)
  (bind _asbp_hero (cast `/Game/Blueprints/BP_Hero` (`GameplayStatics.GetPlayerCharacter` 0)))
  (add `/Game/Blueprints/BP_Hero.Phase2DamDispatcher` _asbp_hero (delegate `Phase2 Damage`)))

(event `Phase2 Damage`
  ;[1 1 1] Add Damage info here
  (`KismetSystemLibrary.PrintString` "Dam Takes Damage"))

(fn `Heal`
  (params (Healing :type "Float (double-precision)"))
  (bind _output_get (set `self.HealthPercent` (+ (`self.Health`) Healing)))
  (bind _output_get_2 (set `self.Health` (`KismetMathLibrary.FClamp` _output_get 0.0 100.0)))
  (set `self.HealthPercent` (/ _output_get_2 100.0)))

(fn `TakeDamage`
  (params (Damage :type "Float (double-precision)"))
  (bind _output_get (set `self.HealthPercent` (- (`self.Health`) Damage)))
  (bind _output_get_2 (set `self.Health` (`KismetMathLibrary.FClamp` _output_get 0.0 100.0)))
  (set `self.HealthPercent` (/ _output_get_2 100.0)))

(fn `UserConstructionScript`)