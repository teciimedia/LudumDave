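; BP_Workbench is a workbench actor where the hero crafts a raft.
; Overlap events on its Trigger component set IsOverlapped while BP_Hero is in range.
; Clicking its 5f component while in range waits briefly, then only prints that the raft is built, while out of range it prints a too-far message.
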(event `self.ReceiveBeginPlay`)

(event `self.Trigger.OnComponentBeginOverlap`
  (params (OverlappedComponent :type "PrimitiveComponent Object Reference") (OtherActor :type "Actor Object Reference") (OtherComp :type "PrimitiveComponent Object Reference") (OtherBodyIndex :type Integer) (bFromSweep :type Boolean) (SweepResult :type "HitResult Structure (by ref)"))
  ;[1 1 1] In range to craft
  (cast `/Game/Blueprints/BP_Hero` OtherActor)
  (set `self.IsOverlapped` true))

(event `self.5f.OnClicked`
  (params (TouchedComponent :type "PrimitiveComponent Object Reference") (ButtonPressed :type "Key Structure"))
  ;[1 1 1] Crafting
  (if (`self.IsOverlapped`)
    (`KismetSystemLibrary.Delay` 2.0)
    (`KismetSystemLibrary.PrintString` "Raft built")
    (else
      (`KismetSystemLibrary.PrintString` "Not close enought"))))

(event `self.Trigger.OnComponentEndOverlap`
  (params (OverlappedComponent :type "PrimitiveComponent Object Reference") (OtherActor :type "Actor Object Reference") (OtherComp :type "PrimitiveComponent Object Reference") (OtherBodyIndex :type Integer))
  ;[1 1 1] Out of range to craft
  (cast `/Game/Blueprints/BP_Hero` OtherActor)
  (set `self.IsOverlapped` false))

(fn `UserConstructionScript`)