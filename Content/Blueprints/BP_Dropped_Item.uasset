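; BP_Dropped_Item is an interactable world item that can be picked up into an inventory.
; On BeginPlay it looks up its ItemData row and applies that row's mesh, scale and materials, writing each material to slot 0.
; InteractWith adds a hardcoded "Log" to the interactor's InventoryComponent, regardless of ItemData, then destroys the actor.
; LookAt returns placeholder test text.
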(event `self.ReceiveBeginPlay`
  (bind (_itemdata_datatable _itemdata_rowname) (break `DataTableRowHandle` (`self.ItemData`)))
  (bind _mesh (`self.Mesh`))
  (bind _returnvalue (`|GetDataTableRow` _itemdata_datatable _itemdata_rowname)
    (:`then`
      (bind (_displayname _description _thumbnail _3dmesh _buycost _sellcost _isstackable _meshscale) (break `/Game/Blueprints/Inventory/ItemStruct` _returnvalue))
      (`StaticMeshComponent.SetStaticMesh` _mesh _3dmesh)
      (`SceneComponent.SetWorldScale3D` _mesh (* (1.0 1.0 1.0) _meshscale))
      (for _array_element (`StaticMesh.StaticMaterials` _3dmesh)
        (`PrimitiveComponent.SetMaterial` (`self.Mesh`) 0 (`.MaterialInterface` (break `StaticMaterial` _array_element)))))))

(fn `InteractWith`
  (params (Interactor :type "/Game/Blueprints/BP_Hero Object Reference"))
  (returns (Success :type Boolean))
  (`/Game/Blueprints/Inventory/InventoryComponent.AddToInventory` (`/Game/Blueprints/BP_Hero.InventoryComponent` Interactor) "Log" 1)
  (`self.K2_DestroyActor`)
  (return true))

(fn `LookAt`
  (params (Observer :type "/Game/Blueprints/BP_Hero Object Reference"))
  (returns (Message :type Text) (Item :type Name))
  (return "Looking atTest" "None"))

(fn `UserConstructionScript`)