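; A clickable pickup actor that adds an item to the player's inventory.
; The construction script picks its static mesh from a Meshes array by Index.
; Clicking the mesh finds the top-level Inventory widget, adds the item by that same Index, then destroys the actor.
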(event `self.StaticMesh.OnClicked`
  (params (TouchedComponent :type "PrimitiveComponent Object Reference") (ButtonPressed :type "Key Structure"))
  (bind _foundwidgets (`WidgetBlueprintLibrary.GetAllWidgetsOfClass` "/Game/UI/inventory.inventory_C"))
  (`/Game/UI/inventory.addItem` (cast `/Game/UI/inventory` (`|GetArrayItem` _foundwidgets) :!pure true) (`self.index`))
  (`self.K2_DestroyActor`))

(fn `UserConstructionScript`
  (`StaticMeshComponent.SetStaticMesh` (`self.StaticMesh`) (`|GetArrayItem` (`self.meshes`) (`self.index`))))