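; BP_PlayerController is a player controller that lets the player switch between beaver, otter and raccoon characters and open a pause menu.
; Keys 1, 2 and 3 each find all actors of the matching animal Blueprint class and possess the first one found, with no validity check.
; The Menu input action creates a new Pause_Menu widget on every press and adds it to the viewport, without pausing the game itself.
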(event `InputAction|Menu`
  (params (Key :type "Key Structure"))
  (:`Pressed`
    (bind _returnvalue (`|CreateWidget` "/Game/UI/Pause_Menu.Pause_Menu_C"))
    (bind _output_get (set `self.PauseMenu` _returnvalue))
    (`UserWidget.AddToViewport` _output_get 0)))

(event `Key|One`
  (params (Key :type "Key Structure"))
  (:`Pressed`
    (bind _outactors (`GameplayStatics.GetAllActorsOfClass` "/Game/Blueprints/BP_Beaver.BP_Beaver_C"))
    (`self.Possess` (`|GetArrayItem` _outactors))))

(event `Key|Two`
  (params (Key :type "Key Structure"))
  (:`Pressed`
    (bind _outactors (`GameplayStatics.GetAllActorsOfClass` "/Game/Blueprints/BP_Otter.BP_Otter_C"))
    (`self.Possess` (`|GetArrayItem` _outactors))))

(event `Key|Three`
  (params (Key :type "Key Structure"))
  (:`Pressed`
    (bind _outactors (`GameplayStatics.GetAllActorsOfClass` "/Game/Blueprints/BP_Racoon.BP_Racoon_C"))
    (`self.Possess` (`|GetArrayItem` _outactors))))

(fn `UserConstructionScript`)